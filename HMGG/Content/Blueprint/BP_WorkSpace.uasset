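; BP_WorkSpace is a work-area trigger that changes the move-to-target state of the object held by BP_MoveHand.
; It caches the first BP_MoveHand in the level on BeginPlay and reads it through a validity-checked GetMoveHand helper.
; WorkSpace begin and end overlaps check the hand's HasObj state, then set opposite SetMoveToTarget values on its DrapObj, without checking which actor overlapped.
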(event `self.ReceiveBeginPlay`
  (`self.InitReference`))

(event `self.WorkSpace.OnComponentBeginOverlap`
  (params (OverlappedComponent :type "PrimitiveComponent Object Reference") (OtherActor :type "Actor Object Reference") (OtherComp :type "PrimitiveComponent Object Reference") (OtherBodyIndex :type Integer) (bFromSweep :type Boolean) (SweepResult :type "HitResult Structure (by ref)"))
  (bind _bpmovehand (`self.GetMoveHand`)
    (:`Is Valid`
      (if (`|EnumEquality` (`/Game/Blueprint/BP_Hand/BP_MoveHand.HasObj` _bpmovehand) "NewEnumerator1")
        (bind _dropobj (`/Game/Blueprint/BP_Hand/BP_MoveHand.GetDrapObj` _bpmovehand))
        (`/Engine/EditorBlueprintResources/StandardMacros.IsValid` _dropobj
          (:`Is Valid`
            (`/Game/Blueprint/BP_DropObj/BP_DropObj.SetMoveToTarget` _dropobj "NewEnumerator0")))))))

(event `self.WorkSpace.OnComponentEndOverlap`
  (params (OverlappedComponent :type "PrimitiveComponent Object Reference") (OtherActor :type "Actor Object Reference") (OtherComp :type "PrimitiveComponent Object Reference") (OtherBodyIndex :type Integer))
  (bind _bpmovehand (`self.GetMoveHand`)
    (:`Is Valid`
      (if (`|EnumEquality` (`/Game/Blueprint/BP_Hand/BP_MoveHand.HasObj` _bpmovehand) "NewEnumerator1")
        (bind _dropobj (`/Game/Blueprint/BP_Hand/BP_MoveHand.GetDrapObj` _bpmovehand))
        (`/Engine/EditorBlueprintResources/StandardMacros.IsValid` _dropobj
          (:`Is Valid`
            (`/Game/Blueprint/BP_DropObj/BP_DropObj.SetMoveToTarget` _dropobj "NewEnumerator1")))))))

(fn `InitReference`
  (bind _outactors (`GameplayStatics.GetAllActorsOfClass` "/Game/Blueprint/BP_Hand/BP_MoveHand.BP_MoveHand_C"))
  (set `self.BpMoveHand` (`KismetArrayLibrary.Array_Get` _outactors)))

(fn `UserConstructionScript`)