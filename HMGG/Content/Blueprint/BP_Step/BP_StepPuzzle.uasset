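; BP_StepPuzzle sequences a two-page step puzzle, left page first and then right.
; Finish events from each page drive the flow: the left clears its page, creates the right page and updates both step tips.
; Finishing the right page shows a PuzzleFinish widget, whose GoToKinectGame event opens StartMap.
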(event `self.ReceiveBeginPlay`
  (add `/Game/Blueprint/BP_Page/BP_PuzzlePage.PageFinishEvent` (`self.PageLeft`) (`|CreateDelegate` :!event `PageFinishEvent_Left`))
  (add `/Game/Blueprint/BP_Page/BP_PuzzlePage.PageFinishEvent` (`self.PageRight`) (`|CreateDelegate` :!event `PageFinishEvent_Right`))
  (`/Game/Blueprint/Bp_Tip/BP_Tips.SetTipStep` (`self.TipLeft`) "NewEnumerator1")
  (`/Game/Blueprint/BP_Page/BP_PuzzlePage.CreatePage` (`self.PageLeft`)))

(event `PageFinishEvent_Left`
  (`/Game/Blueprint/BP_Page/BP_PuzzlePage.ClearPage` (`self.PageLeft`))
  (`/Game/Blueprint/BP_Page/BP_PuzzlePage.CreatePage` (`self.PageRight`))
  (`/Game/Blueprint/Bp_Tip/BP_Tips.SetTipStep` (`self.TipLeft`) "NewEnumerator2")
  (`/Game/Blueprint/Bp_Tip/BP_Tips.SetTipStep` (`self.TipRight`) "NewEnumerator1"))

(event `PageFinishEvent_Right`
  (bind _returnvalue (`|CreateWidget` "/Game/2DAssets/widget/PuzzleFinish.PuzzleFinish_C" (`GameplayStatics.GetPlayerController` 0)))
  (add `/Game/2DAssets/widget/PuzzleFinish.GoToKinectGame` _returnvalue (`|CreateDelegate` :!event `GoToKinectGame`))
  (`UserWidget.AddToViewport` _returnvalue 3))

(event `GoToKinectGame`
  (`GameplayStatics.OpenLevel` "StartMap"))

(fn `UserConstructionScript`)