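; BP_PuzzlePage spawns one page of drop-object puzzle pieces and signals when that page is finished.
; CreatePage spawns a BP_DropObj per DropObj entry at its origin on the XZ plane, passing target point and enable state, and tracking those with valid Paper sprites.
; Tick polls tracked pieces, calling CallPageFinishEvent once none remain enabled.
; Z and C keys trigger creating and clearing the page.
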(event `self.ReceiveTick`
  (params (DeltaSeconds :type "Float (single-precision)"))
  (if (`self.PageBegin`)
    (bind _finish (`self.GetPageFinish`))
    (if _finish
      (set `self.PageBegin` false)
      (`self.PageFinishEvent`))))

(event `Key|Z`
  (params (Key :type "Key Structure" :default "AnyKey"))
  (:`Pressed`
    (`self.CreatePage`)))

(event `Key|C`
  (params (Key :type "Key Structure" :default "AnyKey"))
  (:`Pressed`
    (`self.ClearPage`)))

(fn `ClearPage`
  (for _array_element (`self.tempDropObj`)
    (`self.K2_DestroyActor` _array_element))
  (`KismetArrayLibrary.Array_Clear` (`self.tempDropObj`)))

(fn `CreatePage`
  (locals (Meta :type "/Game/Blueprint/BP_Page/PageMeta Structure"))
  (bind (_paper _origin _target _enable) (break `/Game/Blueprint/BP_Page/PageMeta` (`local.Meta`)))
  (bind (_returnvalue_x _returnvalue_y _returnvalue_z) (`KismetMathLibrary.BreakVector` (`self.K2_GetActorLocation` _target)))
  (bind (_returnvalue_x_2 _returnvalue_y_2 _returnvalue_z_2) (`KismetMathLibrary.BreakVector` (`self.K2_GetActorLocation` (`.Origin_13_81D63D06448244758AD23FB198162393` (break `/Game/Blueprint/BP_Page/PageMeta` (`local.Meta`))))))
  (for _array_element (`self.DropObj`)
    (set `local.Meta` _array_element)
    (bind _returnvalue (`|SpawnActorFromClass` "/Game/Blueprint/BP_DropObj/BP_DropObj.BP_DropObj_C" (`KismetMathLibrary.MakeTransform` (`KismetMathLibrary.MakeVector` _returnvalue_x_2 0.0 _returnvalue_z_2) (struct) (1.0 1.0 1.0)) "Undefined" "OverrideRootScale" (`GameplayStatics.GetPlayerCharacter` 0)))
    (`/Game/Blueprint/BP_DropObj/BP_DropObj.SetSpriteEnable` _returnvalue _enable)
    (set `/Game/Blueprint/BP_DropObj/BP_DropObj.TargetPoint` (`KismetMathLibrary.MakeVector2D` _returnvalue_x _returnvalue_z) _returnvalue)
    (`/Engine/EditorBlueprintResources/StandardMacros.IsValid` _paper
      (:`Is Valid`
        (`/Game/Blueprint/BP_DropObj/BP_DropObj.ResetSpriteOurce` _returnvalue _paper)
        (`KismetArrayLibrary.Array_Add` (`self.tempDropObj`) _returnvalue))))
  (set `self.PageBegin` true))

(fn `GetPageFinish`
  (returns (finish :type Boolean))
  (for _array_element (`self.tempDropObj`)
    (if (`/Game/Blueprint/BP_DropObj/BP_DropObj.isEnable` _array_element)
      (return false)))
  (return true))

(fn `UserConstructionScript`)