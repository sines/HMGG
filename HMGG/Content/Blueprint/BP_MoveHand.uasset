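; Keyboard-driven hand cursor that moves a sprite on the X/Z plane and signals picking up or putting down objects.
; WASD sets a per-tick step that MoveScreen adds to a target point, clamped to fixed screen bounds via identity MapRangeClamped.
; Space swaps palm and fist sprites; each state change fires a pick-up or put-down call based on HasObj.
; A setter and getter hold the dragged object reference.
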(event `self.ReceiveBeginPlay`
  (`self.InitRange`)
  (`self.InitReference`)
  (`self.ChangeHandState` "NewEnumerator0"))

(event `self.ReceiveTick`
  (params (DeltaSeconds :type "Float (single-precision)"))
  (`self.MoveScreen`))

(event `Key|W`
  (params (Key :type "Key Structure" :default "AnyKey"))
  (:`Pressed`
    (`self.SetMove` true 0.0 10.0))
  (:`Released`
    (`self.SetMove` false)))

(event `Key|D`
  (params (Key :type "Key Structure" :default "AnyKey"))
  (:`Pressed`
    (`self.SetMove` true 10.0 0.0))
  (:`Released`
    (`self.SetMove` false)))

(event `Key|A`
  (params (Key :type "Key Structure" :default "AnyKey"))
  (:`Pressed`
    (`self.SetMove` true -10.0 0.0))
  (:`Released`
    (`self.SetMove` false)))

(event `Key|S`
  (params (Key :type "Key Structure" :default "AnyKey"))
  (:`Pressed`
    (`self.SetMove` true 0.0 -10.0))
  (:`Released`
    (`self.SetMove` false)))

(event `Key|SpaceBar`
  (params (Key :type "Key Structure" :default "AnyKey"))
  (:`Pressed`
    (`self.ChangeHandState` "NewEnumerator1"))
  (:`Released`
    (`self.ChangeHandState` "NewEnumerator0")))

(fn `ChangeCover`
  (`/Game/Blueprint/BP_Playpoetry.ChangeCove` (`self.Playpoetry`) "NewEnumerator1"))

(fn `ChangeHandState`
  (params (state :type "/Game/Blueprint/HandStateType Enum"))
  (bind _handsprite (`self.HandSprite`))
  (bind _output_get (set `self.CurrentState` state))
  (switch `/Game/Blueprint/HandStateType` _output_get
    (:`NewEnumerator0`
      (`PaperSpriteComponent.SetSprite` _handsprite "/Game/2DAssets/Sprite/common/Hand/palm_Sprite.palm_Sprite"))
    (:`NewEnumerator1`
      (`PaperSpriteComponent.SetSprite` _handsprite "/Game/2DAssets/Sprite/common/Hand/Fist_Sprite.Fist_Sprite"))
    (:`NewEnumerator2`
      (`PaperSpriteComponent.SetSprite` _handsprite "/Game/2DAssets/Sprite/common/Hand/yeh_Sprite.yeh_Sprite")))
  (`self.MoveScreen`)
  (switch `/Game/Blueprint/HandPickUpState` (`self.HasObj`)
    (:`NewEnumerator0`
      (`self.PickUpObj`))
    (:`NewEnumerator1`
      (`self.PutDownObj`))))

(fn `GetDrapObj`
  (returns (dropObj :type "/Game/2DAssets/Sprite/common/DynaSprite/BP_DropObj Object Reference"))
  (return (`self.DrapObj`)))

(fn `InitRange`
  (bind (_despoint_x _despoint_y) (`KismetMathLibrary.BreakVector2D` (`self.DesPoint`)))
  (bind _boundaxlex_min (break `/Game/Blueprint/Bound2D` (`self.BoundAxleX`)))
  (bind _boundaxley_min (break `/Game/Blueprint/Bound2D` (`self.BoundAxleY`)))
  (set `self.BoundAxleX` (make `/Game/Blueprint/Bound2D` -936.0 932.0))
  (set `self.BoundAxleY` (make `/Game/Blueprint/Bound2D` -515.0 520.0))
  (set `self.DesPoint` (`KismetMathLibrary.MakeVector2D` _boundaxlex_min _boundaxley_min))
  (`SceneComponent.K2_SetWorldLocation` (`self.Root`) (`KismetMathLibrary.MakeVector` _despoint_x 0.08 _despoint_y) false false))

(fn `InitReference`)

(fn `MoveScreen`
  (bind (_boundaxlex_min _boundaxlex_max) (break `/Game/Blueprint/Bound2D` (`self.BoundAxleX`)))
  (bind (_despoint_x _despoint_y) (`KismetMathLibrary.BreakVector2D` (`self.DesPoint`)))
  (bind (_despoint_x_2 _despoint_y_2) (`KismetMathLibrary.BreakVector2D` (`self.DesPoint`)))
  (bind (_boundaxley_min _boundaxley_max) (break `/Game/Blueprint/Bound2D` (`self.BoundAxleY`)))
  (if (`self.IsMove`)
    (set `self.DesPoint` (`KismetMathLibrary.MakeVector2D` (`KismetMathLibrary.MapRangeClamped` (+ _despoint_x (`self.Axle_x`)) _boundaxlex_min _boundaxlex_max _boundaxlex_min _boundaxlex_max) (`KismetMathLibrary.MapRangeClamped` (+ _despoint_y (`self.Axle_z`)) _boundaxley_min _boundaxley_max _boundaxley_min _boundaxley_max)))
    (`SceneComponent.K2_SetWorldLocation` (`self.Root`) (`KismetMathLibrary.MakeVector` _despoint_x_2 0.08 _despoint_y_2) false false)))

(fn `SetDrapObj`
  (params (DrapObj :type "/Game/2DAssets/Sprite/common/DynaSprite/BP_DropObj Object Reference"))
  (`/Engine/EditorBlueprintResources/StandardMacros.IsValid` DrapObj
    (:`Is Valid`
      (set `self.DrapObj` DrapObj))))

(fn `SetMove`
  (params (IsMove :type Boolean) (x :type "Float (double-precision)") (z :type "Float (double-precision)"))
  (set `self.IsMove` IsMove)
  (set `self.Axle_x` x)
  (set `self.Axle_z` z))

(fn `UserConstructionScript`)