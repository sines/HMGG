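; StartButton is a 2D actor that plays a one-shot start-button flipbook animation.
; On BeginPlay, InitStartButtonAni rewinds the animation, stops it and turns off looping.
; Pressing the 1 key plays it from the start at normal rate, and finishing only prints a debug "Hello", with no game-start logic attached.
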(event `self.ReceiveBeginPlay`
  (`self.InitStartButtonAni`))

(event `Key|One`
  (params (Key :type "Key Structure" :default "AnyKey"))
  (bind _startbuttonani (`self.StartButtonAni`))
  (:`Pressed`
    (`PaperFlipbookComponent.SetPlayRate` _startbuttonani 1.0)
    (`PaperFlipbookComponent.PlayFromStart` _startbuttonani)))

(event `self.StartButtonAni.OnFinishedPlaying`
  (`KismetSystemLibrary.PrintString` "Hello"))

(fn `InitStartButtonAni`
  (bind _startbuttonani (`self.StartButtonAni`))
  (`PaperFlipbookComponent.SetPlaybackPosition` _startbuttonani 0.0 true)
  (`PaperFlipbookComponent.Stop` _startbuttonani)
  (`PaperFlipbookComponent.SetLooping` _startbuttonani false))

(fn `UserConstructionScript`)