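; BP_DropObj is a 2D sprite object that a BP_MoveHand actor can pick up and put down.
; It binds to the hand's pickup and putdown events, attaching to it when overlapped and detaching on release.
; After release, a timeline slides it in the XZ plane to its target point or its starting position, depending on the target state.
; Keys 1 and 2 also trigger those moves directly.
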(event `self.ReceiveBeginPlay`
  (`self.InitPoint`)
  (`self.InitReference`))

(event `self.ReceiveTick`
  (params (DeltaSeconds :type "Float (single-precision)")))

(event `PlayMoveSprite`
  (params (target :type "Vector2D Structure"))
  (bind (_returnvalue_x _returnvalue_y _returnvalue_z) (`KismetMathLibrary.BreakVector` (`SceneComponent.K2_GetComponentLocation` (`self.Root`))))
  (bind _returnvalue (`KismetMathLibrary.MakeVector2D` _returnvalue_x _returnvalue_z))
  (if (`self.isFinished`)
    (set `self.TempTarget` target)
    (set `self.isFinished` false)
    (bind (_direction _tc) (`Timeline|tc` :!via `PlayFromStart`)
      (:`Update`
        (`self.GotoPoint` (+ (* (- (`self.TempTarget`) _returnvalue) _tc) _returnvalue)))
      (:`Finished`
        (set `self.isFinished` true)))))

(event `Key|One`
  (params (Key :type "Key Structure" :default "AnyKey"))
  (:`Pressed`
    (`self.PlayMoveSprite` (`self.SrcPoint`))))

(event `Key|Two`
  (params (Key :type "Key Structure" :default "AnyKey"))
  (:`Pressed`
    (`self.PlayMoveSprite` (`self.TargetPoint`))))

(event `self.PaperSprite.OnComponentBeginOverlap`
  (params (OverlappedComponent :type "PrimitiveComponent Object Reference") (OtherActor :type "Actor Object Reference") (OtherComp :type "PrimitiveComponent Object Reference") (OtherBodyIndex :type Integer) (bFromSweep :type Boolean) (SweepResult :type "HitResult Structure (by ref)"))
  (if (== OtherActor (`self.bp_hand`))
    (set `self.IntoSprite` true)))

(event `self.PaperSprite.OnComponentEndOverlap`
  (params (OverlappedComponent :type "PrimitiveComponent Object Reference") (OtherActor :type "Actor Object Reference") (OtherComp :type "PrimitiveComponent Object Reference") (OtherBodyIndex :type Integer))
  (if (== OtherActor (`self.bp_hand`))
    (set `self.IntoSprite` false)))

(event `PickUp`
  (if (`self.IntoSprite`)
    (if (`|EnumEquality` (`/Game/Blueprint/BP_MoveHand.CurrentState` (`self.bp_hand`)) "NewEnumerator1")
      (`self.BindHand`)
      (set `self.CurrentState` "NewEnumerator0")
      (set `/Game/Blueprint/BP_MoveHand.HasObj` "NewEnumerator1" (`self.bp_hand`)))))

(event `put down`
  (if (`|EnumEquality` (`self.CurrentState`) "NewEnumerator0")
    (`self.UnBindHand`)
    (set `self.CurrentState` "NewEnumerator1")
    (set `/Game/Blueprint/BP_MoveHand.HasObj` "NewEnumerator0" (`self.bp_hand`))
    (`self.MovetoPoint`)))

(fn `BindHand`
  (`SceneComponent.K2_AttachToComponent` (`self.Root`) (`/Game/Blueprint/BP_MoveHand.Root` (`self.bp_hand`)) "None" "KeepWorld" "KeepRelative" "KeepWorld" true))

(fn `GotoPoint`
  (params (point :type "Vector2D Structure"))
  (`SceneComponent.K2_SetWorldLocation` (`self.Root`) (`KismetMathLibrary.MakeVector` point_X 0.0 point_Y) false false))

(fn `InitPoint`
  (bind (_returnvalue_x _returnvalue_y _returnvalue_z) (`KismetMathLibrary.BreakVector` (`SceneComponent.K2_GetComponentLocation` (`self.Root`))))
  (set `self.SrcPoint` (`KismetMathLibrary.MakeVector2D` _returnvalue_x _returnvalue_z)))

(fn `InitReference`
  (bind _outactors (`GameplayStatics.GetAllActorsOfClass` "/Game/Blueprint/BP_MoveHand.BP_MoveHand_C"))
  (bind _output_get (set `self.bp_hand` (`KismetArrayLibrary.Array_Get` _outactors)))
  (add `/Game/Blueprint/BP_MoveHand.PickUpObj` _output_get (`|CreateDelegate` :!event `PickUp`))
  (add `/Game/Blueprint/BP_MoveHand.PutDownObj` _output_get (`|CreateDelegate` :!event `put down`)))

(fn `InitState`
  (set `self.isFinished` true)
  (set `self.IntoSprite` false)
  (set `self.CurrentState` "NewEnumerator1")
  (set `self.CurrentTargetState` "NewEnumerator1"))

(fn `MovetoPoint`
  (switch `/Game/2DAssets/Sprite/common/DynaSprite/GoToType` (`self.CurrentTargetState`)
    (:`NewEnumerator0`
      (`self.PlayMoveSprite` (`self.TargetPoint`)))
    (:`NewEnumerator1`
      (`self.PlayMoveSprite` (`self.SrcPoint`)))))

(fn `SetTarget`
  (params (target :type "/Game/2DAssets/Sprite/common/DynaSprite/GoToType Enum"))
  (set `self.CurrentTargetState` target))

(fn `UnBindHand`
  (`SceneComponent.DetachFromParent` (`self.Root`) true false))

(fn `UserConstructionScript`
  (set `self.isFinished` true)
  (`self.InitState`))