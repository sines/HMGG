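; Start button actor that opens the Puzzle level when the player's MoveHand confirms it with a closed hand.
; Overlapping the animation component with MoveHand, or pressing the 1 key, plays the button animation once at triple speed; ending an overlap resets it and disarms the button.
; Finishing the animation sets the Jump flag, after which Tick polls the hand state and loads the level once it reads Closed.
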(event `self.ReceiveBeginPlay`
  (`self.InitStartButtonAni`))

(event `Key|One`
  (params (Key :type "Key Structure" :default "AnyKey"))
  (:`Pressed`
    (`self.PlayStartButton`)))

(event `self.ReceiveTick`
  (params (DeltaSeconds :type "Float (single-precision)"))
  (bind _movehand (`self.MoveHand`))
  (if (`self.Jump`)
    (`/Engine/EditorBlueprintResources/StandardMacros.IsValid` _movehand
      (:`Is Valid`
        (if (`|EnumEquality` (`/Game/Blueprints/BP_Hand/BP_MoveHand.CurrentHandState` _movehand) "Closed")
          (`GameplayStatics.OpenLevel` "Puzzle"))))))

(event `self.StartButtonAni.OnFinishedPlaying`
  (set `self.Jump` true))

(event `self.StartButtonAni.OnComponentBeginOverlap`
  (params (OverlappedComponent :type "PrimitiveComponent Object Reference") (OtherActor :type "Actor Object Reference") (OtherComp :type "PrimitiveComponent Object Reference") (OtherBodyIndex :type Integer) (bFromSweep :type Boolean) (SweepResult :type "HitResult Structure (by ref)"))
  (if (== OtherActor (`self.MoveHand`))
    (`self.PlayStartButton`)))

(event `self.StartButtonAni.OnComponentEndOverlap`
  (params (OverlappedComponent :type "PrimitiveComponent Object Reference") (OtherActor :type "Actor Object Reference") (OtherComp :type "PrimitiveComponent Object Reference") (OtherBodyIndex :type Integer))
  (`self.StopStartButton`)
  (set `self.Jump` false))

(fn `InitStartButtonAni`
  (bind _startbuttonani (`self.StartButtonAni`))
  (`PaperFlipbookComponent.SetPlaybackPosition` _startbuttonani 0.0 true)
  (`PaperFlipbookComponent.Stop` _startbuttonani)
  (`PaperFlipbookComponent.SetLooping` _startbuttonani false))

(fn `PlayStartButton`
  (bind _startbuttonani (`self.StartButtonAni`))
  (`PaperFlipbookComponent.SetPlayRate` _startbuttonani 3.0)
  (`PaperFlipbookComponent.PlayFromStart` _startbuttonani))

(fn `StopStartButton`
  (`self.InitStartButtonAni`))

(fn `UserConstructionScript`)