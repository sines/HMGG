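; Sound tip actor that plays a configured sound while a filtered actor is inside its sphere bound.
; On entry it tells SoundTipsManager to stop all sounds before playing; on exit it stops and calls CallCallBackground.
; BeginPlay assigns the sound with back-to-back fade in and out, but InitRefece leaves SoundTipsManager set to None despite an actor lookup.
; Helper functions expose playback state and manual play or stop.
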(event `self.ReceiveBeginPlay`
  (`self.InitAudioInfo`)
  (`self.InitRefece`))

(event `self.ReceiveTick`
  (params (DeltaSeconds :type "Float (single-precision)")))

(event `self.SphereCollisionBound.OnComponentBeginOverlap`
  (params (OverlappedComponent :type "PrimitiveComponent Object Reference") (OtherActor :type "Actor Object Reference") (OtherComp :type "PrimitiveComponent Object Reference") (OtherBodyIndex :type Integer) (bFromSweep :type Boolean) (SweepResult :type "HitResult Structure (by ref)"))
  (if (== OtherActor (`self.ActorFiltr`))
    (`/Game/Blueprints/BP_Sound/Bp/Bp_SoundTipsManager.StopAllSound` (`self.SoundTipsManager`))
    (`AudioComponent.Play` (`self.Audio`) 0.0)))

(event `self.SphereCollisionBound.OnComponentEndOverlap`
  (params (OverlappedComponent :type "PrimitiveComponent Object Reference") (OtherActor :type "Actor Object Reference") (OtherComp :type "PrimitiveComponent Object Reference") (OtherBodyIndex :type Integer))
  (if (== OtherActor (`self.ActorFiltr`))
    (`AudioComponent.Stop` (`self.Audio`))
    (`self.CallBackground`)))

(event `self.Audio.OnAudioFinished`)

(fn `GetIsPlaying`
  (returns (IsPlaying :type Boolean))
  (bind _output_get (set `self.IsPlaying` (`AudioComponent.IsPlaying` (`self.Audio`))))
  (return _output_get))

(fn `InitAudioInfo`
  (`AudioComponent.SetSound` (`self.Audio`) (`self.Sound`))
  (`AudioComponent.FadeIn` (`self.Audio`) 0.3 1.0 0.0)
  (`AudioComponent.FadeOut` (`self.Audio`) 0.1 0.3))

(fn `InitRefece`
  (bind _outactors (`GameplayStatics.GetAllActorsOfClass` null))
  (set `self.SoundTipsManager` null))

(fn `PlayAudio`
  (params (play :type Boolean))
  (if play
    (`AudioComponent.Play` (`self.Audio`) 0.0)
    (set `self.IsPlaying` true)
    (else
      (`AudioComponent.Stop` (`self.Audio`))
      (set `self.IsPlaying` false))))

(fn `SysRadius`)

(fn `UserConstructionScript`)