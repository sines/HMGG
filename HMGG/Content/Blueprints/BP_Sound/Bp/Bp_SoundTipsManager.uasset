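; Manager actor that coordinates the level's background music and all Bp_SoundTip actors.
; On BeginPlay it sets up and plays the background track, gathers every sound tip, and binds each tip's background callback to replay the music from the start.
; Helper functions push an actor filter to all tips, stop every tip and the music, or stop everything and switch the music to NextSound.
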(event `self.ReceiveBeginPlay`
  (`self.InitAudioInfo`)
  (`self.InitReference`)
  (`self.PlayBackgroundMsic`)
  (for _array_element (`self.SoundTipsList`)
    (add `/Game/Blueprints/BP_Sound/Bp/Bp_SoundTip.CallBackground` _array_element (delegate `PlayBackgroundMsic`))))

(event `PlayBackgroundMsic`
  (`AudioComponent.Play` (`self.BackgroundMusic`) 0.0))

(fn `InitAudioInfo`
  (`AudioComponent.SetSound` (`self.BackgroundMusic`) (`self.BackgroundSound`))
  (`AudioComponent.FadeIn` (`self.BackgroundMusic`) 0.3 1.0 0.0)
  (`AudioComponent.FadeOut` (`self.BackgroundMusic`) 0.1 0.3))

(fn `InitReference`
  (bind _outactors (`GameplayStatics.GetAllActorsOfClass` "/Game/Blueprints/BP_Sound/Bp/Bp_SoundTip.Bp_SoundTip_C"))
  (set `self.SoundTipsList` _outactors))

(fn `PlayNextSound`
  (`self.StopAllSound`)
  (`AudioComponent.SetSound` (`self.BackgroundMusic`) (`self.NextSound`))
  (`AudioComponent.Play` (`self.BackgroundMusic`) 0.0))

(fn `SetAllFilte`
  (params (filtr :type "Actor Object Reference"))
  (for _array_element (`self.SoundTipsList`)
    (set `/Game/Blueprints/BP_Sound/Bp/Bp_SoundTip.ActorFiltr` filtr _array_element)))

(fn `StopAllSound`
  (for _array_element (`self.SoundTipsList`)
    (`/Game/Blueprints/BP_Sound/Bp/Bp_SoundTip.PlayAudio` _array_element false))
  (`AudioComponent.Stop` (`self.BackgroundMusic`)))

(fn `UserConstructionScript`)