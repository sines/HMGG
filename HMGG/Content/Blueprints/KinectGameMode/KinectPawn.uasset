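; KinectPawn is a pawn that polls Kinect body tracking and records detected players in its Connect slot array.
; Each Tick writes tracked bodies, with their body indices, into successive slots until the array is full.
; It clears every slot when nobody is tracked, or the second slot when only one body is.
; A TimeOut function that reopens StartMap after over ten minutes without a body exists but is never called.
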(event `self.ReceiveBeginPlay`
  (set `self.StartConnectTime` (`KismetMathLibrary.Now`)))

(event `self.ReceiveTick`
  (params (DeltaSeconds :type "Float (single-precision)"))
  (set `self.index` 0)
  (bind _out (`KinectPluginFunctionLibrary.GetKinectTrackedBodies`))
  (for (_array_element _array_index) _out
    (if _array_element
      (`KismetArrayLibrary.Array_Set` (`self.connect`) (`self.index`) (make `/Game/Blueprints/KinectGameMode/KinectBodyIndex` true _array_index))
      (set `self.index` (+ (`self.index`) 1))
      (if (>= (`self.index`) (`KismetArrayLibrary.Array_Length` (`self.connect`)))
        (break))))
  (switch `int` (`self.index`)
    (:`0`
      (`self.ClearState`))
    (:`1`
      (`KismetArrayLibrary.Array_Set` (`self.connect`) 1 (struct)))))

(fn `ClearState`
  (for (_ _array_index) (`self.connect`)
    (`KismetArrayLibrary.Array_Set` (`self.connect`) _array_index (struct))))

(fn `TimeOut`
  (bind (_out _returnvalue) (`KinectPluginFunctionLibrary.GetFirstActiveKinectBody`))
  (if _returnvalue
    (set `self.StartConnectTime` (`KismetMathLibrary.Now`))
    (elif (> (`KismetMathLibrary.GetMinutes` (- (`KismetMathLibrary.Now`) (`self.StartConnectTime`))) 10)
      (`GameplayStatics.OpenLevel` "StartMap"))))

(fn `UserConstructionScript`)