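; BP_DropObj is a 2D sprite object that the BP_MoveHand actor can pick up, carry and drop.
; Overlap registers it with an empty hand, whose bound events attach it when closed and detach it when open.
; On release, a timeline slides it across the XZ plane back to its start point or to its target.
; The target case also adjusts scale, disables overlaps and signals that the move to target is finished.
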(event `self.ReceiveBeginPlay`
  (`self.InitPoint`)
  (`self.InitReference`))

(event `self.ReceiveTick`
  (params (DeltaSeconds :type "Float (single-precision)")))

(event `PlayMoveSprite`
  (params (target :type "Vector2D Structure") (IsTarget :type Boolean))
  (bind (_returnvalue_x _returnvalue_y _returnvalue_z) (`KismetMathLibrary.BreakVector` (`SceneComponent.K2_GetComponentLocation` (`self.Root`))))
  (bind _returnvalue (`KismetMathLibrary.MakeVector2D` _returnvalue_x _returnvalue_z))
  (if (`self.isMoveFinished`)
    (set `self.TempTarget` target)
    (set `self.isMoveFinished` false)
    (bind (_direction _tc) (`Timeline|tc` :!via `PlayFromStart`)
      (:`Update`
        (`self.GotoPoint` (+ (* (- (`self.TempTarget`) _returnvalue) _tc) _returnvalue))
        (if IsTarget
          (bind (_returnvalue_x_2 _returnvalue_y_2 _returnvalue_z_2) (`KismetMathLibrary.BreakVector` (+ (`self.GetActorScale3D` self) _tc)))
          (`self.Scale` self (`KismetMathLibrary.MakeVector` (`KismetMathLibrary.MapRangeClamped` _returnvalue_x_2 0.0 1.0 0.0 1.0) (`KismetMathLibrary.MapRangeClamped` _returnvalue_y_2 0.0 1.0 0.0 1.0) (`KismetMathLibrary.MapRangeClamped` _returnvalue_z_2 0.0 1.0 0.0 1.0)))))
      (:`Finished`
        (set `self.isMoveFinished` true)))))

(event `self.PaperSprite.OnComponentBeginOverlap`
  (params (OverlappedComponent :type "PrimitiveComponent Object Reference") (OtherActor :type "Actor Object Reference") (OtherComp :type "PrimitiveComponent Object Reference") (OtherBodyIndex :type Integer) (bFromSweep :type Boolean) (SweepResult :type "HitResult Structure (by ref)"))
  (bind _bp_hand (`self.bp_hand`))
  (if (== OtherActor _bp_hand)
    (set `self.IntoSprite` true)
    (if (`|EnumEquality` (`/Game/Blueprints/BP_Hand/BP_MoveHand.HasObj` _bp_hand) "NewEnumerator0")
      (`/Game/Blueprints/BP_Hand/BP_MoveHand.SetDrapObj` _bp_hand self))))

(event `self.PaperSprite.OnComponentEndOverlap`
  (params (OverlappedComponent :type "PrimitiveComponent Object Reference") (OtherActor :type "Actor Object Reference") (OtherComp :type "PrimitiveComponent Object Reference") (OtherBodyIndex :type Integer))
  (if (== OtherActor (`self.bp_hand`))
    (set `self.IntoSprite` false)))

(event `PickUp`
  (if (`self.IntoSprite`)
    (if (`|EnumEquality` (`/Game/Blueprints/BP_Hand/BP_MoveHand.CurrentHandState` (`self.bp_hand`)) "Closed")
      (`self.BindHand`)
      (set `self.CurrentState` "NewEnumerator0")
      (set `/Game/Blueprints/BP_Hand/BP_MoveHand.HasObj` "NewEnumerator1" (`self.bp_hand`)))))

(event `put down`
  (if (`|EnumEquality` (`/Game/Blueprints/BP_Hand/BP_MoveHand.CurrentHandState` (`self.bp_hand`)) "Open")
    (`self.UnBindHand`)
    (set `self.CurrentState` "NewEnumerator1")
    (set `/Game/Blueprints/BP_Hand/BP_MoveHand.HasObj` "NewEnumerator0" (`self.bp_hand`))
    (`self.MovetoPoint`)))

(fn `BindHand`
  (`SceneComponent.K2_AttachToComponent` (`self.Root`) (`/Game/Blueprints/BP_Hand/BP_MoveHand.Root` (`self.bp_hand`)) "None" "KeepWorld" "KeepRelative" "KeepWorld" true))

(fn `GotoPoint`
  (params (point :type "Vector2D Structure"))
  (`SceneComponent.K2_SetWorldLocation` (`self.Root`) (`KismetMathLibrary.MakeVector` point_X 0.0 point_Y) false false))

(fn `InitPoint`
  (bind (_returnvalue_x _returnvalue_y _returnvalue_z) (`KismetMathLibrary.BreakVector` (`SceneComponent.K2_GetComponentLocation` (`self.Root`))))
  (set `self.SrcPoint` (`KismetMathLibrary.MakeVector2D` _returnvalue_x _returnvalue_z)))

(fn `InitReference`
  (bind _outactors (`GameplayStatics.GetAllActorsOfClass` "/Game/Blueprints/BP_Hand/BP_MoveHand.BP_MoveHand_C"))
  (bind _output_get (set `self.bp_hand` (`KismetArrayLibrary.Array_Get` _outactors)))
  (`PrimitiveComponent.SetTranslucentSortPriority` (`/Game/Blueprints/BP_Hand/BP_MoveHand.HandSprite` _output_get) 1)
  (add `/Game/Blueprints/BP_Hand/BP_MoveHand.PickUpObj` _output_get (`|CreateDelegate` :!event `PickUp`))
  (add `/Game/Blueprints/BP_Hand/BP_MoveHand.PutDownObj` _output_get (`|CreateDelegate` :!event `put down`)))

(fn `InitState`
  (set `self.isMoveFinished` true)
  (set `self.IntoSprite` false)
  (set `self.CurrentState` "NewEnumerator1")
  (set `self.CurrentTargetState` "NewEnumerator1"))

(fn `MovetoPoint`
  (switch `/Game/Blueprints/BP_DropObj/GoToType` (`self.CurrentTargetState`)
    (:`NewEnumerator0`
      (`self.PlayMoveSprite` (`self.TargetPoint`) true)
      (set `PrimitiveComponent.bGenerateOverlapEvents` false (`self.PaperSprite`))
      (set `self.isEnable` false)
      (`self.ObjectMoveToTargetFinish`))
    (:`NewEnumerator1`
      (`self.PlayMoveSprite` (`self.SrcPoint`)))))

(fn `ResetSpriteOurce`
  (params (Paper :type "PaperSprite Object Reference"))
  (returns (Success :type Boolean))
  (bind _returnvalue (`PaperSpriteComponent.SetSprite` (`self.PaperSprite`) Paper))
  (return _returnvalue))

(fn `Scale`
  (params (scale :type "Vector Structure"))
  (`SceneComponent.SetWorldScale3D` (`self.Root`) scale))

(fn `SetMoveToTarget`
  (params (target :type "/Game/Blueprints/BP_DropObj/GoToType Enum"))
  (set `self.CurrentTargetState` target))

(fn `SetSpriteEnable`
  (params (Enable :type Boolean))
  (set `PrimitiveComponent.bGenerateOverlapEvents` Enable (`self.PaperSprite`))
  (set `self.isEnable` Enable))

(fn `UnBindHand`
  (`SceneComponent.DetachFromParent` (`self.Root`) true false))

(fn `UserConstructionScript`
  (set `self.isMoveFinished` true)
  (`self.InitState`))