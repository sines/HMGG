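; Introduction actor that visualizes selected Kinect skeleton joints in 3D, with text readouts of their coordinates.
; Each tick, while an active body is found, a helper moves the head, ankle, wrist and spine-base meshes to their joint positions and updates their coordinate text.
; All labels, including hand-state texts, are then yawed toward the player's pawn, using the spine-base mesh as the shared reference point.
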(event `self.ReceiveTick`
  (params (DeltaSeconds :type "Float (single-precision)"))
  (bind (_out _returnvalue) (`KinectPluginFunctionLibrary.GetFirstActiveKinectBody`))
  (if _returnvalue
    (`self.UpdateIncicatorMesh` "Head" (`self.MeshHead`) (`self.TextHeadCoord`))
    (`self.UpdateIncicatorMesh` "AnkleLeft" (`self.MeshLAnkle`) (`self.TextLAnkleCoord`))
    (`self.UpdateIncicatorMesh` "AnkleRight" (`self.MeshRAnkle`) (`self.TextRAnkleCoord`))
    (`self.UpdateIncicatorMesh` "AnkleRight" (`self.MeshRAnkle`) (`self.TextRAnkleCoord`))
    (`self.UpdateIncicatorMesh` "WristLeft" (`self.MeshLWrist`) (`self.TextLWristCoord`))
    (`self.UpdateIncicatorMesh` "WristRight" (`self.MeshRWrist`) (`self.TextRWristCoord`))
    (`self.UpdateIncicatorMesh` "SpineBase" (`self.MeshSpinebase`) (`self.TextSpinebaseCoord`))
    (`SceneComponent.K2_SetWorldRotation` (`self.TextSpinebaseCoord`) (`KismetMathLibrary.MakeRotator` 0.0 0.0 (.yaw (`KismetMathLibrary.FindLookAtRotation` (`SceneComponent.K2_GetComponentLocation` (`self.MeshSpinebase`)) (`self.K2_GetActorLocation` (`Controller.K2_GetPawn` (`GameplayStatics.GetPlayerController` 0)))))) false false)
    (`SceneComponent.K2_SetWorldRotation` (`self.TextSpinebase`) (`KismetMathLibrary.MakeRotator` 0.0 0.0 (.yaw (`KismetMathLibrary.FindLookAtRotation` (`SceneComponent.K2_GetComponentLocation` (`self.MeshSpinebase`)) (`self.K2_GetActorLocation` (`Controller.K2_GetPawn` (`GameplayStatics.GetPlayerController` 0)))))) false false)
    (`SceneComponent.K2_SetWorldRotation` (`self.TextHeadCoord`) (`KismetMathLibrary.MakeRotator` 0.0 0.0 (.yaw (`KismetMathLibrary.FindLookAtRotation` (`SceneComponent.K2_GetComponentLocation` (`self.MeshSpinebase`)) (`self.K2_GetActorLocation` (`Controller.K2_GetPawn` (`GameplayStatics.GetPlayerController` 0)))))) false false)
    (`SceneComponent.K2_SetWorldRotation` (`self.TextHead`) (`KismetMathLibrary.MakeRotator` 0.0 0.0 (.yaw (`KismetMathLibrary.FindLookAtRotation` (`SceneComponent.K2_GetComponentLocation` (`self.MeshSpinebase`)) (`self.K2_GetActorLocation` (`Controller.K2_GetPawn` (`GameplayStatics.GetPlayerController` 0)))))) false false)
    (`SceneComponent.K2_SetWorldRotation` (`self.TextRHandState`) (`KismetMathLibrary.MakeRotator` 0.0 0.0 (.yaw (`KismetMathLibrary.FindLookAtRotation` (`SceneComponent.K2_GetComponentLocation` (`self.MeshSpinebase`)) (`self.K2_GetActorLocation` (`Controller.K2_GetPawn` (`GameplayStatics.GetPlayerController` 0)))))) false false)
    (`SceneComponent.K2_SetWorldRotation` (`self.TextRWristCoord`) (`KismetMathLibrary.MakeRotator` 0.0 0.0 (.yaw (`KismetMathLibrary.FindLookAtRotation` (`SceneComponent.K2_GetComponentLocation` (`self.MeshSpinebase`)) (`self.K2_GetActorLocation` (`Controller.K2_GetPawn` (`GameplayStatics.GetPlayerController` 0)))))) false false)
    (`SceneComponent.K2_SetWorldRotation` (`self.TextRWrist`) (`KismetMathLibrary.MakeRotator` 0.0 0.0 (.yaw (`KismetMathLibrary.FindLookAtRotation` (`SceneComponent.K2_GetComponentLocation` (`self.MeshSpinebase`)) (`self.K2_GetActorLocation` (`Controller.K2_GetPawn` (`GameplayStatics.GetPlayerController` 0)))))) false false)
    (`SceneComponent.K2_SetWorldRotation` (`self.TextLHandState`) (`KismetMathLibrary.MakeRotator` 0.0 0.0 (.yaw (`KismetMathLibrary.FindLookAtRotation` (`SceneComponent.K2_GetComponentLocation` (`self.MeshSpinebase`)) (`self.K2_GetActorLocation` (`Controller.K2_GetPawn` (`GameplayStatics.GetPlayerController` 0)))))) false false)
    (`SceneComponent.K2_SetWorldRotation` (`self.TextLWristCoord`) (`KismetMathLibrary.MakeRotator` 0.0 0.0 (.yaw (`KismetMathLibrary.FindLookAtRotation` (`SceneComponent.K2_GetComponentLocation` (`self.MeshSpinebase`)) (`self.K2_GetActorLocation` (`Controller.K2_GetPawn` (`GameplayStatics.GetPlayerController` 0)))))) false false)
    (`SceneComponent.K2_SetWorldRotation` (`self.TextLWrist`) (`KismetMathLibrary.MakeRotator` 0.0 0.0 (.yaw (`KismetMathLibrary.FindLookAtRotation` (`SceneComponent.K2_GetComponentLocation` (`self.MeshSpinebase`)) (`self.K2_GetActorLocation` (`Controller.K2_GetPawn` (`GameplayStatics.GetPlayerController` 0)))))) false false)
    (`SceneComponent.K2_SetWorldRotation` (`self.TextRAnkleCoord`) (`KismetMathLibrary.MakeRotator` 0.0 0.0 (.yaw (`KismetMathLibrary.FindLookAtRotation` (`SceneComponent.K2_GetComponentLocation` (`self.MeshSpinebase`)) (`self.K2_GetActorLocation` (`Controller.K2_GetPawn` (`GameplayStatics.GetPlayerController` 0)))))) false false)
    (`SceneComponent.K2_SetWorldRotation` (`self.TextRAnkle`) (`KismetMathLibrary.MakeRotator` 0.0 0.0 (.yaw (`KismetMathLibrary.FindLookAtRotation` (`SceneComponent.K2_GetComponentLocation` (`self.MeshSpinebase`)) (`self.K2_GetActorLocation` (`Controller.K2_GetPawn` (`GameplayStatics.GetPlayerController` 0)))))) false false)
    (`SceneComponent.K2_SetWorldRotation` (`self.TextLAnkleCoord`) (`KismetMathLibrary.MakeRotator` 0.0 0.0 (.yaw (`KismetMathLibrary.FindLookAtRotation` (`SceneComponent.K2_GetComponentLocation` (`self.MeshSpinebase`)) (`self.K2_GetActorLocation` (`Controller.K2_GetPawn` (`GameplayStatics.GetPlayerController` 0)))))) false false)
    (`SceneComponent.K2_SetWorldRotation` (`self.TextLAnkle`) (`KismetMathLibrary.MakeRotator` 0.0 0.0 (.yaw (`KismetMathLibrary.FindLookAtRotation` (`SceneComponent.K2_GetComponentLocation` (`self.MeshSpinebase`)) (`self.K2_GetActorLocation` (`Controller.K2_GetPawn` (`GameplayStatics.GetPlayerController` 0)))))) false false)))

(fn `UpdateIncicatorMesh`
  (params (JointType :type "EFLKinect_JointType Enum") (Mesh :type "SceneComponent Object Reference") (TextCoord :type "TextRenderComponent Object Reference"))
  (bind _returnvalue (`KinectPluginFunctionLibrary.GetJointPosition` (`self.KinectBody`) JointType))
  (`SceneComponent.K2_SetRelativeLocation` Mesh _returnvalue false false)
  (`TextRenderComponent.K2_SetText` TextCoord (`KismetTextLibrary.Conv_VectorToText` _returnvalue)))

(fn `UserConstructionScript`)