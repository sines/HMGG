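; BP_StepKinectGame tracks task progress in the Kinect game and shows the game-over screen once every task is done.
; On BeginPlay it binds to the move-to-target-finish event of each entry in Tasks.
; A task event fades Tips, increments a counter and adds the KinectGameOver widget when the count reaches the task total.
; Space opens StartMap and R reloads the KinectGame level.
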(event `self.ReceiveBeginPlay`
  (for _array_element (`self.Tasks`)
    (add `/Game/Blueprints/BP_CollisionMoveObj/BP_CollisionMoveObj.ObjectMoveToTargetFinish` _array_element (`|CreateDelegate` :!event `task`))))

(event `task`
  (`/Game/Blueprints/Bp_Tip/BP_Tips.AlphaDec` (`self.tips`) 0.0)
  (set `self.TaskCount` (+ (`self.TaskCount`) 1))
  (if (>= (`self.TaskCount`) (`KismetArrayLibrary.Array_Length` (`self.Tasks`)))
    (bind _returnvalue (`|CreateWidget` "/Game/2DAssets/widget/KinectGameOver.KinectGameOver_C" (`GameplayStatics.GetPlayerController` 0)))
    (`UserWidget.AddToViewport` _returnvalue 0)))

(event `Key|SpaceBar`
  (params (Key :type "Key Structure" :default "AnyKey"))
  (:`Pressed`
    (`GameplayStatics.OpenLevel` "StartMap")))

(event `Key|R`
  (params (Key :type "Key Structure" :default "AnyKey"))
  (:`Pressed`
    (`GameplayStatics.OpenLevel` "KinectGame")))

(fn `UserConstructionScript`)