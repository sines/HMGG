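; BP_StepPuzzle sequences a two-page puzzle, left page then right, and leads on to the KinectGame level.
; It binds each page's finish events to update the matching tip's step.
; The left page's delayed finish clears it and creates the right page, whose delayed finish shows a PuzzleFinish widget bound to open KinectGame.
; Space, R and T jump directly to the StartMap, Puzzle and KinectGame levels.
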(event `self.ReceiveBeginPlay`
  (bind _pageright (`self.PageRight`))
  (add `/Game/Blueprints/BP_Page/BP_PuzzlePage.PageDelayFinishEvent` (`self.PageLeft`) (`|CreateDelegate` :!event `PageDelayFinishEvent_Left`))
  (add `/Game/Blueprints/BP_Page/BP_PuzzlePage.PageTiFinishEvent` (`self.PageLeft`) (`|CreateDelegate` :!event `PageTiFinishEvent_Left`))
  (add `/Game/Blueprints/BP_Page/BP_PuzzlePage.PageDelayFinishEvent` _pageright (`|CreateDelegate` :!event `PageDelayFinishEvent_Right`))
  (add `/Game/Blueprints/BP_Page/BP_PuzzlePage.PageTiFinishEvent` _pageright (`|CreateDelegate` :!event `PageTiFinishEvent_Right`))
  (`/Game/Blueprints/Bp_Tip/BP_Tips.SetTipStep` (`self.TipLeft`) "NewEnumerator0")
  (`/Game/Blueprints/BP_Page/BP_PuzzlePage.CreatePage` (`self.PageLeft`)))

(event `PageDelayFinishEvent_Left`
  (`/Game/Blueprints/BP_Page/BP_PuzzlePage.ClearPage` (`self.PageLeft`))
  (`/Game/Blueprints/BP_Page/BP_PuzzlePage.CreatePage` (`self.PageRight`))
  (`/Game/Blueprints/Bp_Tip/BP_Tips.SetTipStep` (`self.TipLeft`) "NewEnumerator2")
  (`/Game/Blueprints/Bp_Tip/BP_Tips.SetTipStep` (`self.TipRight`) "NewEnumerator1"))

(event `PageDelayFinishEvent_Right`
  (bind _returnvalue (`|CreateWidget` "/Game/2DAssets/widget/PuzzleFinish.PuzzleFinish_C" (`GameplayStatics.GetPlayerController` 0)))
  (add `/Game/2DAssets/widget/PuzzleFinish.GoToKinectGame` _returnvalue (`|CreateDelegate` :!event `GoToKinectGame`))
  (`UserWidget.AddToViewport` _returnvalue 3))

(event `PageTiFinishEvent_Right`
  (`/Game/Blueprints/Bp_Tip/BP_Tips.SetTipStep` (`self.TipRight`) "NewEnumerator2"))

(event `PageTiFinishEvent_Left`
  (`/Game/Blueprints/Bp_Tip/BP_Tips.SetTipStep` (`self.TipLeft`) "NewEnumerator2"))

(event `GoToKinectGame`
  (`GameplayStatics.OpenLevel` "KinectGame"))

(event `Key|SpaceBar`
  (params (Key :type "Key Structure" :default "AnyKey"))
  (:`Pressed`
    (`GameplayStatics.OpenLevel` "StartMap")))

(event `Key|R`
  (params (Key :type "Key Structure" :default "AnyKey"))
  (:`Pressed`
    (`GameplayStatics.OpenLevel` "Puzzle")))

(event `Key|T`
  (params (Key :type "Key Structure" :default "AnyKey"))
  (:`Pressed`
    (`GameplayStatics.OpenLevel` "KinectGame")))

(fn `UserConstructionScript`)