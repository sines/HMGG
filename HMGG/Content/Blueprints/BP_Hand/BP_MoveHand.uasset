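; Sprite hand cursor that moves within screen bounds on the XZ plane, driven by keyboard or Kinect as selected by IsKey.
; Kinect maps the right hand's offset from an origin, reset by the Lasso gesture, onto those bounds.
; Hand state swaps the palm, fist or lasso sprite; open and closed also call pick-up or put-down based on HasObj.
; An older inline Kinect version remains unconnected in the EventGraph.
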(event `self.ReceiveEndPlay`
  (params (EndPlayReason :type "EEndPlayReason Enum" :default "Destroyed")))

(event `self.ReceiveBeginPlay`
  (`self.InitRange`)
  (`self.InitReference`)
  (`self.ChangeHandState` "Open")
  (set `self.HasObj` "NewEnumerator0"))

(event `self.ReceiveTick`
  (params (DeltaSeconds :type "Float (single-precision)"))
  (if (`self.IsKey`)
    (`self.MoveScreen`)
    (else
      (bind (_out _returnvalue) (`KinectPluginFunctionLibrary.GetFirstActiveKinectBody`))
      (if _returnvalue
        (`self.KinectChangeHandState` _out)
        (`self.KinectChangeHandMove` _out)))))

(event `Key|F`
  (params (Key :type "Key Structure" :default "AnyKey"))
  (:`Pressed`
    (set `self.IsMove` true))
  (:`Released`
    (set `self.IsMove` false)))

(event `Key|W`
  (params (Key :type "Key Structure" :default "AnyKey"))
  (:`Pressed`
    (`self.SetMove` true 0.0 10.0))
  (:`Released`
    (`self.SetMove` false)))

(event `Key|D`
  (params (Key :type "Key Structure" :default "AnyKey"))
  (:`Pressed`
    (`self.SetMove` true 10.0 0.0))
  (:`Released`
    (`self.SetMove` false)))

(event `Key|A`
  (params (Key :type "Key Structure" :default "AnyKey"))
  (:`Pressed`
    (`self.SetMove` true -10.0 0.0))
  (:`Released`
    (`self.SetMove` false)))

(event `Key|S`
  (params (Key :type "Key Structure" :default "AnyKey"))
  (:`Pressed`
    (`self.SetMove` true 0.0 -10.0))
  (:`Released`
    (`self.SetMove` false)))

(event `Key|SpaceBar`
  (params (Key :type "Key Structure" :default "AnyKey"))
  (:`Pressed`
    (`self.ChangeHandState` "Closed"))
  (:`Released`
    (`self.ChangeHandState` "Open")))

(fn `ChangeCover`
  (`/Game/Blueprints/BP_Playpoetry/BP_Playpoetry.ChangeCove` (`self.Playpoetry`) "NewEnumerator1"))

(fn `ChangeHandState`
  (params (state :type "EFLKinect_HandState Enum"))
  (bind _handsprite (`self.HandSprite`))
  (set `self.CurrentHandState` state)
  (switch `EFLKinect_HandState` state
    (:`Open`
      (`PaperSpriteComponent.SetSprite` _handsprite "/Game/2DAssets/Sprite/common/Hand/palm_Sprite.palm_Sprite")
      (`self.MoveScreen` :!label _label)
      (switch `/Game/Blueprints/BP_Hand/HandPickUpState` (`self.HasObj`)
        (:`NewEnumerator0`
          (`self.PickUpObj`))
        (:`NewEnumerator1`
          (`self.PutDownObj`))))
    (:`Closed`
      (`PaperSpriteComponent.SetSprite` _handsprite "/Game/2DAssets/Sprite/common/Hand/Fist_Sprite.Fist_Sprite")
      (goto _label))
    (:`Lasso`
      (`PaperSpriteComponent.SetSprite` _handsprite "/Game/2DAssets/Sprite/common/Hand/yeh_Sprite.yeh_Sprite")
      (`self.MoveScreen`))))

(fn `GetDrapObj`
  (returns (dropObj :type "/Game/Blueprints/BP_DropObj/BP_DropObj Object Reference"))
  (return (`self.DrapObj`)))

(fn `InitRange`
  (bind (_despoint_x _despoint_y) (`KismetMathLibrary.BreakVector2D` (`self.DesPoint`)))
  (bind _boundaxlex_min (break `/Game/Blueprints/BP_Hand/Bound2D` (`self.BoundAxleX`)))
  (bind _boundaxley_min (break `/Game/Blueprints/BP_Hand/Bound2D` (`self.BoundAxleY`)))
  (set `self.BoundAxleX` (make `/Game/Blueprints/BP_Hand/Bound2D` -936.0 932.0))
  (set `self.BoundAxleY` (make `/Game/Blueprints/BP_Hand/Bound2D` -515.0 520.0))
  (set `self.DesPoint` (`KismetMathLibrary.MakeVector2D` _boundaxlex_min _boundaxley_min))
  (`SceneComponent.K2_SetWorldLocation` (`self.Root`) (`KismetMathLibrary.MakeVector` _despoint_x 0.08 _despoint_y) false false))

(fn `InitReference`)

(fn `KinectChangeHandMove`
  (params (KinectBody :type "FLKinect_Body Structure"))
  (bind (_despoint_x _despoint_y) (`KismetMathLibrary.BreakVector2D` (`self.DesPoint`)))
  (bind (_boundaxlex_min _boundaxlex_max) (break `/Game/Blueprints/BP_Hand/Bound2D` (`self.BoundAxleX`)))
  (bind (_boundaxley_min _boundaxley_max) (break `/Game/Blueprints/BP_Hand/Bound2D` (`self.BoundAxleY`)))
  (bind (_x _y) (`KismetMathLibrary.BreakVector2D` (- (`KismetMathLibrary.MakeVector2D` (.x (`KinectPluginFunctionLibrary.GetJointPosition` KinectBody "HandRight")) (.z (`KinectPluginFunctionLibrary.GetJointPosition` KinectBody "HandRight"))) (`self.SrcPoint`))))
  (if (`|EnumEquality` (`KinectPluginFunctionLibrary.GetTrackingState` KinectBody "HandRight") "Tracking")
    (set `self.DesPoint` (`KismetMathLibrary.MakeVector2D` (`KismetMathLibrary.Lerp` _boundaxlex_min _boundaxlex_max (`KismetMathLibrary.NormalizeToRange` _x -40.0 40.0)) (`KismetMathLibrary.Lerp` _boundaxley_min _boundaxley_max (`KismetMathLibrary.NormalizeToRange` _y -40.0 40.0))))
    (`SceneComponent.K2_SetWorldLocation` (`self.Root`) (`KismetMathLibrary.MakeVector` _despoint_x 0.1 _despoint_y) false false)
    (`PrimitiveComponent.SetTranslucentSortPriority` (`self.HandSprite`) 3)))

(fn `KinectChangeHandState`
  (params (KinectBody :type "FLKinect_Body Structure"))
  (bind ((`HandRightState` _handrightstate)) (break `FLKinect_Body` KinectBody))
  (if (`|EnumEquality` (`KinectPluginFunctionLibrary.GetTrackingState` KinectBody "HandRight") "Tracking")
    (`|ExecutionSequence`
      (:`then_0`
        (`|MultiGate` false :!label _label
          (:`Out 0`
            (switch `EFLKinect_HandState` _handrightstate
              (:`Open`
                (`self.ChangeHandState` "Open"))
              (:`Closed`
                (`self.ChangeHandState` "Closed"))
              (:`Lasso`
                (`self.ChangeHandState` "Lasso")
                (set `self.SrcPoint` (`KismetMathLibrary.MakeVector2D` (.x (`KinectPluginFunctionLibrary.GetJointPosition` KinectBody "HandRight")) (.z (`KinectPluginFunctionLibrary.GetJointPosition` KinectBody "HandRight")))))))))
      (:`then_1`
        (if (not (`|EnumEquality` _handrightstate (`self.CurrentHandState`)))
          (goto _label :!via `Reset`))))))

(fn `MoveScreen`
  (returns (P :type "Vector2D Structure"))
  (bind (_boundaxlex_min _boundaxlex_max) (break `/Game/Blueprints/BP_Hand/Bound2D` (`self.BoundAxleX`)))
  (bind (_despoint_x _despoint_y) (`KismetMathLibrary.BreakVector2D` (`self.DesPoint`)))
  (bind (_despoint_x_2 _despoint_y_2) (`KismetMathLibrary.BreakVector2D` (`self.DesPoint`)))
  (bind (_boundaxley_min _boundaxley_max) (break `/Game/Blueprints/BP_Hand/Bound2D` (`self.BoundAxleY`)))
  (if (`self.IsMove`)
    (bind _output_get (set `self.DesPoint` (`KismetMathLibrary.MakeVector2D` (`KismetMathLibrary.MapRangeClamped` (+ _despoint_x (`self.Axle_x`)) _boundaxlex_min _boundaxlex_max _boundaxlex_min _boundaxlex_max) (`KismetMathLibrary.MapRangeClamped` (+ _despoint_y (`self.Axle_z`)) _boundaxley_min _boundaxley_max _boundaxley_min _boundaxley_max))))
    (`SceneComponent.K2_SetWorldLocation` (`self.Root`) (`KismetMathLibrary.MakeVector` _despoint_x_2 0.1 _despoint_y_2) false false)
    (`PrimitiveComponent.SetTranslucentSortPriority` (`self.HandSprite`) 3)
    (return (`KismetMathLibrary.MakeVector2D` _despoint_x_2 _despoint_y_2))
    (else
      (return _output_get))))

(fn `SetDrapObj`
  (params (DrapObj :type "/Game/Blueprints/BP_DropObj/BP_DropObj Object Reference"))
  (`/Engine/EditorBlueprintResources/StandardMacros.IsValid` DrapObj
    (:`Is Valid`
      (set `self.DrapObj` DrapObj))))

(fn `SetMove`
  (params (IsMove :type Boolean) (x :type "Float (double-precision)") (z :type "Float (double-precision)"))
  (set `self.IsMove` IsMove)
  (set `self.Axle_x` x)
  (set `self.Axle_z` z))

(fn `UserConstructionScript`)