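; BP_Playpoetry is an actor that plays a poetry display through its Playpoetry widget and switches it when Kinect activation occurs.
; On BeginPlay, it binds to the first BP_MoveHand's Kinect activation and starts the ShowPoetry timeline, which drives the widget's Play each update.
; An activation during playback is remembered through IsJump and applied after the timeline finishes and a short delay; later activations switch immediately.
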(event `self.ReceiveBeginPlay`
  (`self.InitReference`)
  (add `/Game/Blueprints/BP_Hand/BP_MoveHand.KinectActivation` (`self.Bp_MoveHand`) (delegate `KinectAdvice`))
  (set `self.IsFinished` false)
  (bind (_direction _tc) (`Timeline|ShowPoetry`)
    (:`Update`
      (`/Game/2DAssets/widget/Playpoetry.Play` (`self.GetPlaypoetry`) _tc))
    (:`Finished`
      (set `self.IsFinished` true)
      (if (`self.IsJump`)
        (`KismetSystemLibrary.Delay` 3.0)
        (`self.ChangeCove` "NewEnumerator1")))))

(event `KinectAdvice`
  (`self.ChangeCove` "NewEnumerator1"))

(fn `ChangeCove`
  (params (playPoetry :type "/Game/Blueprints/BP_Playpoetry/UIPlaypoetryType Enum"))
  (set `self.IsJump` true)
  (if (`self.IsFinished`)
    (`/Game/2DAssets/widget/Playpoetry.ChangePlaypoetry` (`self.GetPlaypoetry`) playPoetry)))

(fn `InitReference`
  (bind _outactors (`GameplayStatics.GetAllActorsOfClass` "/Game/Blueprints/BP_Hand/BP_MoveHand.BP_MoveHand_C"))
  (set `self.Bp_MoveHand` (`KismetArrayLibrary.Array_Get` _outactors)))

(fn `UserConstructionScript`)