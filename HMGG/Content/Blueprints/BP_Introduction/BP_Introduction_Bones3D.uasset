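; Kinect introduction Blueprint that shows the first active tracked body as per-joint indicator meshes with text labels.
; Each tick, UpdateIncicatorMesh moves core, arm and leg meshes to their joint positions, zeroing Y to flatten the skeleton onto the XZ plane.
; Labels yaw from the spine base toward the player's pawn.
; Coordinate labels receive a constant zero vector instead of joint positions, and hand-state labels are only rotated.
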(event `self.ReceiveTick`
  (params (DeltaSeconds :type "Float (single-precision)"))
  (bind (_out _returnvalue) (`KinectPluginFunctionLibrary.GetFirstActiveKinectBody`))
  (if _returnvalue
    (set `self.KinectBody` _out)
    ;[1 1 1] Core
    (`self.UpdateIncicatorMesh` "SpineBase" (`self.MeshSpineBase`) (`self.TextSpinebaseCoord`))
    (`self.UpdateIncicatorMesh` "SpineMid" (`self.MeshSpineMid`))
    (`self.UpdateIncicatorMesh` "Neck" (`self.MeshNeck`))
    (`self.UpdateIncicatorMesh` "Head" (`self.MeshHead`) (`self.TextHeadCoord`))
    ;[1 1 1] Arms
    (`self.UpdateIncicatorMesh` "HandLeft" (`self.MeshLHand`))
    (`self.UpdateIncicatorMesh` "ShoulderLeft" (`self.MeshLShoulder`))
    (`self.UpdateIncicatorMesh` "ElbowLeft" (`self.MeshLElbow`))
    (`self.UpdateIncicatorMesh` "WristLeft" (`self.MeshLWrist`) (`self.TextLWristCoord`))
    (`self.UpdateIncicatorMesh` "ElbowRight" (`self.MeshRElbow`))
    (`self.UpdateIncicatorMesh` "WristRight" (`self.MeshRWrist`) (`self.TextRWristCoord`))
    (`self.UpdateIncicatorMesh` "ShoulderRight" (`self.MeshRShoulder`))
    (`self.UpdateIncicatorMesh` "HandRight" (`self.MeshRHand`))
    ;[1 1 1] Legs
    (`self.UpdateIncicatorMesh` "HipLeft" (`self.MeshLHip`))
    (`self.UpdateIncicatorMesh` "KneeLeft" (`self.MeshLKnee`))
    (`self.UpdateIncicatorMesh` "AnkleLeft" (`self.MeshLAnkle`) (`self.TextLAnkleCoord`))
    (`self.UpdateIncicatorMesh` "KneeRight" (`self.MeshRKnee`))
    (`self.UpdateIncicatorMesh` "AnkleRight" (`self.MeshRAnkle`) (`self.TextRAnkleCoord`))
    (`self.UpdateIncicatorMesh` "HipRight" (`self.MeshRHip`))
    (`SceneComponent.K2_SetWorldRotation` (`self.TextSpinebaseCoord`) (`KismetMathLibrary.MakeRotator` 0.0 0.0 (.yaw (`KismetMathLibrary.FindLookAtRotation` (`SceneComponent.K2_GetComponentLocation` (`self.MeshSpineBase`)) (`self.K2_GetActorLocation` (`Controller.K2_GetPawn` (`GameplayStatics.GetPlayerController` 0)))))) false false)
    (`SceneComponent.K2_SetWorldRotation` (`self.TextSpinebase`) (`KismetMathLibrary.MakeRotator` 0.0 0.0 (.yaw (`KismetMathLibrary.FindLookAtRotation` (`SceneComponent.K2_GetComponentLocation` (`self.MeshSpineBase`)) (`self.K2_GetActorLocation` (`Controller.K2_GetPawn` (`GameplayStatics.GetPlayerController` 0)))))) false false)
    (`SceneComponent.K2_SetWorldRotation` (`self.TextHeadCoord`) (`KismetMathLibrary.MakeRotator` 0.0 0.0 (.yaw (`KismetMathLibrary.FindLookAtRotation` (`SceneComponent.K2_GetComponentLocation` (`self.MeshSpineBase`)) (`self.K2_GetActorLocation` (`Controller.K2_GetPawn` (`GameplayStatics.GetPlayerController` 0)))))) false false)
    (`SceneComponent.K2_SetWorldRotation` (`self.TextHead`) (`KismetMathLibrary.MakeRotator` 0.0 0.0 (.yaw (`KismetMathLibrary.FindLookAtRotation` (`SceneComponent.K2_GetComponentLocation` (`self.MeshSpineBase`)) (`self.K2_GetActorLocation` (`Controller.K2_GetPawn` (`GameplayStatics.GetPlayerController` 0)))))) false false)
    (`SceneComponent.K2_SetWorldRotation` (`self.TextRHandState`) (`KismetMathLibrary.MakeRotator` 0.0 0.0 (.yaw (`KismetMathLibrary.FindLookAtRotation` (`SceneComponent.K2_GetComponentLocation` (`self.MeshSpineBase`)) (`self.K2_GetActorLocation` (`Controller.K2_GetPawn` (`GameplayStatics.GetPlayerController` 0)))))) false false)
    (`SceneComponent.K2_SetWorldRotation` (`self.TextRWristCoord`) (`KismetMathLibrary.MakeRotator` 0.0 0.0 (.yaw (`KismetMathLibrary.FindLookAtRotation` (`SceneComponent.K2_GetComponentLocation` (`self.MeshSpineBase`)) (`self.K2_GetActorLocation` (`Controller.K2_GetPawn` (`GameplayStatics.GetPlayerController` 0)))))) false false)
    (`SceneComponent.K2_SetWorldRotation` (`self.TextRWrist`) (`KismetMathLibrary.MakeRotator` 0.0 0.0 (.yaw (`KismetMathLibrary.FindLookAtRotation` (`SceneComponent.K2_GetComponentLocation` (`self.MeshSpineBase`)) (`self.K2_GetActorLocation` (`Controller.K2_GetPawn` (`GameplayStatics.GetPlayerController` 0)))))) false false)
    (`SceneComponent.K2_SetWorldRotation` (`self.TextLHandState`) (`KismetMathLibrary.MakeRotator` 0.0 0.0 (.yaw (`KismetMathLibrary.FindLookAtRotation` (`SceneComponent.K2_GetComponentLocation` (`self.MeshSpineBase`)) (`self.K2_GetActorLocation` (`Controller.K2_GetPawn` (`GameplayStatics.GetPlayerController` 0)))))) false false)
    (`SceneComponent.K2_SetWorldRotation` (`self.TextLWristCoord`) (`KismetMathLibrary.MakeRotator` 0.0 0.0 (.yaw (`KismetMathLibrary.FindLookAtRotation` (`SceneComponent.K2_GetComponentLocation` (`self.MeshSpineBase`)) (`self.K2_GetActorLocation` (`Controller.K2_GetPawn` (`GameplayStatics.GetPlayerController` 0)))))) false false)
    (`SceneComponent.K2_SetWorldRotation` (`self.TextLWrist`) (`KismetMathLibrary.MakeRotator` 0.0 0.0 (.yaw (`KismetMathLibrary.FindLookAtRotation` (`SceneComponent.K2_GetComponentLocation` (`self.MeshSpineBase`)) (`self.K2_GetActorLocation` (`Controller.K2_GetPawn` (`GameplayStatics.GetPlayerController` 0)))))) false false)
    (`SceneComponent.K2_SetWorldRotation` (`self.TextRAnkleCoord`) (`KismetMathLibrary.MakeRotator` 0.0 0.0 (.yaw (`KismetMathLibrary.FindLookAtRotation` (`SceneComponent.K2_GetComponentLocation` (`self.MeshSpineBase`)) (`self.K2_GetActorLocation` (`Controller.K2_GetPawn` (`GameplayStatics.GetPlayerController` 0)))))) false false)
    (`SceneComponent.K2_SetWorldRotation` (`self.TextRAnkle`) (`KismetMathLibrary.MakeRotator` 0.0 0.0 (.yaw (`KismetMathLibrary.FindLookAtRotation` (`SceneComponent.K2_GetComponentLocation` (`self.MeshSpineBase`)) (`self.K2_GetActorLocation` (`Controller.K2_GetPawn` (`GameplayStatics.GetPlayerController` 0)))))) false false)
    (`SceneComponent.K2_SetWorldRotation` (`self.TextLAnkleCoord`) (`KismetMathLibrary.MakeRotator` 0.0 0.0 (.yaw (`KismetMathLibrary.FindLookAtRotation` (`SceneComponent.K2_GetComponentLocation` (`self.MeshSpineBase`)) (`self.K2_GetActorLocation` (`Controller.K2_GetPawn` (`GameplayStatics.GetPlayerController` 0)))))) false false)
    (`SceneComponent.K2_SetWorldRotation` (`self.TextLAnkle`) (`KismetMathLibrary.MakeRotator` 0.0 0.0 (.yaw (`KismetMathLibrary.FindLookAtRotation` (`SceneComponent.K2_GetComponentLocation` (`self.MeshSpineBase`)) (`self.K2_GetActorLocation` (`Controller.K2_GetPawn` (`GameplayStatics.GetPlayerController` 0)))))) false false)))

(fn `UpdateIncicatorMesh`
  (params (JointType :type "EFLKinect_JointType Enum") (Mesh :type "SceneComponent Object Reference") (TextCoord :type "TextRenderComponent Object Reference"))
  (`/Engine/EditorBlueprintResources/StandardMacros.IsValid` Mesh
    (:`Is Valid`
      (`SceneComponent.K2_SetRelativeLocation` Mesh (* (`KinectPluginFunctionLibrary.GetJointPosition` (`self.KinectBody`) JointType) (1.0 0.0 1.0)) false false)
      (`/Engine/EditorBlueprintResources/StandardMacros.IsValid` TextCoord
        (:`Is Valid`
          (`TextRenderComponent.K2_SetText` TextCoord (`KismetTextLibrary.Conv_VectorToText` (0.0 0.0 0.0))))))))

(fn `UserConstructionScript`)