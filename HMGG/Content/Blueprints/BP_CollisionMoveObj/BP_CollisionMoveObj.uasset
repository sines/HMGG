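; BP_CollisionMoveObj is a Paper2D sprite object that glides across the XZ plane to TargetPoint and signals when it arrives.
; MovetoPoint reads the target state and starts PlayMoveSprite, whose timeline blends from the current location each update, guarded by IsMoveFinished.
; The Target state also resets scale and rotation and disables sprite overlaps.
; Go Back still heads to TargetPoint, as the saved SrcPoint is never read here.
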(event `self.ReceiveBeginPlay`
  (`self.InitPoint`)
  (`self.InitReference`))

(event `self.ReceiveTick`
  (params (DeltaSeconds :type "Float (single-precision)")))

(event `PlayMoveSprite`
  (params (IsTarget :type Boolean))
  (bind (_returnvalue_x _returnvalue_y _returnvalue_z) (`KismetMathLibrary.BreakVector` (`SceneComponent.K2_GetComponentLocation` (`self.Root`))))
  (bind (_returnvalue_x_2 _returnvalue_y_2 _returnvalue_z_2) (`KismetMathLibrary.BreakVector` (`self.K2_GetActorLocation` (`self.TargetPoint`))))
  (bind _returnvalue (`KismetMathLibrary.MakeVector2D` _returnvalue_x _returnvalue_z))
  (if (`self.isMoveFinished`)
    (set `self.TempTarget` (`KismetMathLibrary.MakeVector2D` _returnvalue_x_2 _returnvalue_z_2))
    (set `self.isMoveFinished` false)
    (bind (_direction _tc) (`Timeline|tc` :!via `PlayFromStart`)
      (:`Update`
        (`self.GotoPoint` (+ (* (- (`self.TempTarget`) _returnvalue) _tc) _returnvalue))
        (if IsTarget
          (bind (_returnvalue_x_3 _returnvalue_y_3 _returnvalue_z_3) (`KismetMathLibrary.BreakVector` (+ (`self.GetActorScale3D` self) _tc)))
          (`self.Scale` self (`KismetMathLibrary.MakeVector` (`KismetMathLibrary.MapRangeClamped` _returnvalue_x_3 0.0 1.0 0.0 1.0) (`KismetMathLibrary.MapRangeClamped` _returnvalue_y_3 0.0 1.0 0.0 1.0) (`KismetMathLibrary.MapRangeClamped` _returnvalue_z_3 0.0 1.0 0.0 1.0)))
          (`self.K2_SetActorRotation` :`self` self)))
      (:`Finished`
        (set `self.isMoveFinished` true)
        (`self.ObjectMoveToTargetFinish`)))))

(fn `GotoPoint`
  (params (point :type "Vector2D Structure"))
  (`SceneComponent.K2_SetWorldLocation` (`self.Root`) (`KismetMathLibrary.MakeVector` point_X 0.0 point_Y) false false))

(fn `InitPoint`
  (bind (_returnvalue_x _returnvalue_y _returnvalue_z) (`KismetMathLibrary.BreakVector` (`SceneComponent.K2_GetComponentLocation` (`self.Root`))))
  (set `self.SrcPoint` (`KismetMathLibrary.MakeVector2D` _returnvalue_x _returnvalue_z)))

(fn `InitReference`)

(fn `InitState`
  (set `self.isMoveFinished` true))

(fn `MovetoPoint`
  (switch `/Game/Blueprints/BP_DropObj/GoToType` (`self.CurrentTargetState`)
    (:`NewEnumerator0`
      (`self.PlayMoveSprite` true)
      (set `PrimitiveComponent.bGenerateOverlapEvents` false (`self.PaperSprite`))
      (set `self.isEnable` false))
    (:`NewEnumerator1`
      (`self.PlayMoveSprite` false))))

(fn `ResetSpriteOurce`
  (params (Paper :type "PaperSprite Object Reference"))
  (returns (Success :type Boolean))
  (bind _returnvalue (`PaperSpriteComponent.SetSprite` (`self.PaperSprite`) Paper))
  (return _returnvalue))

(fn `Scale`
  (params (scale :type "Vector Structure"))
  (`SceneComponent.SetWorldScale3D` (`self.Root`) scale))

(fn `SetMoveToTarget`
  (params (target :type "/Game/Blueprints/BP_DropObj/GoToType Enum"))
  (set `self.CurrentTargetState` target))

(fn `SetSpriteEnable`
  (params (Enable :type Boolean))
  (set `PrimitiveComponent.bGenerateOverlapEvents` Enable (`self.PaperSprite`))
  (set `self.isEnable` Enable))

(fn `UserConstructionScript`
  (set `self.isMoveFinished` true)
  (`self.InitState`))