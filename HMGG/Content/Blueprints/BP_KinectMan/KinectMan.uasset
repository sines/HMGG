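; KinectMan is a Blueprint for experimenting with Kinect body tracking and debug drawing, and appears unfinished.
; BeginPlay fetches the first active Kinect body but uses none of its data.
; Loops that would read positions from six body slots and draw boxes over an array are disconnected.
; The 1 key calls the debug box draw directly, using the element of that unexecuted loop as its center.
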(event EventBeginPlay
  (bind _out (Class|KinectPluginFunctionLibrary|GetFirstActiveKinectBody)))

(event Collision|EventActorBeginOverlap
  (params (OtherActor :type Actor%20Object%20Reference)))

(event EventTick
  (params (DeltaSeconds :type Float%20%28single-precision%29)))

(event Input|KeyboardEvents|1
  (params (Key :type Key%20Structure :default "AnyKey"))
  (:Pressed
    (Rendering|Debug|DrawDebugBox :Center (stale _array_element) :Extent "1.000000,1.000000,1.000000")))

(fn ConstructionScript)