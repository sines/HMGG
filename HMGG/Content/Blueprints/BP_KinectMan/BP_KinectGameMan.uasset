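; Kinect-based 2D paper-sprite character whose hands trigger PlayMoveSprite on any BP_CollisionMoveObj they overlap.
; Helper functions flatten joint positions onto planes and remap limb angles into clamped sprite pitch for shoulders, elbows and legs.
; The pose chain that moves joint meshes and rotates those sprites from the first active body is disconnected and never runs.
; Tick only loops over tracked bodies with an empty body, so hand overlaps are the only active behavior.
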(event `self.ReceiveTick`
  (params (DeltaSeconds :type "Float (single-precision)"))
  (bind _out (`KinectPluginFunctionLibrary.GetKinectTrackedBodies`))
  (for _ _out
    _))

(event `self.RightHand.OnComponentBeginOverlap`
  (params (OverlappedComponent :type "PrimitiveComponent Object Reference") (OtherActor :type "Actor Object Reference") (OtherComp :type "PrimitiveComponent Object Reference") (OtherBodyIndex :type Integer) (bFromSweep :type Boolean) (SweepResult :type "HitResult Structure (by ref)"))
  (if (== (`GameplayStatics.GetObjectClass` OtherActor) "/Game/Blueprints/BP_CollisionMoveObj/BP_CollisionMoveObj.BP_CollisionMoveObj_C")
    (bind _asbp_collision_move_obj (cast `/Game/Blueprints/BP_CollisionMoveObj/BP_CollisionMoveObj` OtherActor))
    (`/Game/Blueprints/BP_CollisionMoveObj/BP_CollisionMoveObj.PlayMoveSprite` _asbp_collision_move_obj true)))

(event `self.lefthand.OnComponentBeginOverlap`
  (params (OverlappedComponent :type "PrimitiveComponent Object Reference") (OtherActor :type "Actor Object Reference") (OtherComp :type "PrimitiveComponent Object Reference") (OtherBodyIndex :type Integer) (bFromSweep :type Boolean) (SweepResult :type "HitResult Structure (by ref)"))
  (if (== (`GameplayStatics.GetObjectClass` OtherActor) "/Game/Blueprints/BP_CollisionMoveObj/BP_CollisionMoveObj.BP_CollisionMoveObj_C")
    (bind _asbp_collision_move_obj (cast `/Game/Blueprints/BP_CollisionMoveObj/BP_CollisionMoveObj` OtherActor))
    (`/Game/Blueprints/BP_CollisionMoveObj/BP_CollisionMoveObj.PlayMoveSprite` _asbp_collision_move_obj true)))

(fn `GetLeftElbowOrientation`
  (params (body :type "FLKinect_Body Structure (by ref)"))
  (returns (Rotator :type "Rotator Structure"))
  (bind _returnvalue (`KismetMathLibrary.Normal` (1.0 1.0 0.0)))
  (bind (_returnvalue_roll _returnvalue_pitch _returnvalue_yaw) (`KismetMathLibrary.BreakRotator` (`KismetMathLibrary.Conv_VectorToRotator` (- (- (* (`KinectPluginFunctionLibrary.GetJointPosition` body "ElbowLeft") _returnvalue) (* (`KinectPluginFunctionLibrary.GetJointPosition` body "WristLeft") _returnvalue)) (- (* (`KinectPluginFunctionLibrary.GetJointPosition` body "ElbowLeft") _returnvalue) (* (`KinectPluginFunctionLibrary.GetJointPosition` body "ShoulderLeft") _returnvalue))))))
  (return (`KismetMathLibrary.MakeRotator` 0.0 (`KismetMathLibrary.MapRangeClamped` _returnvalue_yaw 0.0 120.0 30.0 150.0))))

(fn `GetLeftLegOrientation`
  (params (body :type "FLKinect_Body Structure (by ref)"))
  (returns (ReturnValue :type "Rotator Structure"))
  (bind _returnvalue (`KismetMathLibrary.Normal` (1.0 0.0 1.0)))
  (bind (_returnvalue_roll _returnvalue_pitch _returnvalue_yaw) (`KismetMathLibrary.BreakRotator` (`KismetMathLibrary.FindLookAtRotation` (* (`KinectPluginFunctionLibrary.GetJointPosition` body "HipLeft") _returnvalue) (* (`KinectPluginFunctionLibrary.GetJointPosition` body "KneeLeft") _returnvalue))))
  (return (`KismetMathLibrary.MakeRotator` _returnvalue_roll (`KismetMathLibrary.MapRangeClamped` _returnvalue_pitch -85.0 -20.0 0.0 40.0) _returnvalue_yaw)))

(fn `GetLeftShoulderOrientation`
  (params (body :type "FLKinect_Body Structure (by ref)"))
  (returns (ReturnValue :type "Rotator Structure"))
  (bind _returnvalue (`KismetMathLibrary.Normal` (1.0 0.0 1.0)))
  (bind (_returnvalue_roll _returnvalue_pitch _returnvalue_yaw) (`KismetMathLibrary.BreakRotator` (`KismetMathLibrary.FindLookAtRotation` (* (`KinectPluginFunctionLibrary.GetJointPosition` body "ElbowLeft") _returnvalue) (* (`KinectPluginFunctionLibrary.GetJointPosition` body "ShoulderLeft") _returnvalue))))
  (return (`KismetMathLibrary.MakeRotator` _returnvalue_roll (`KismetMathLibrary.MapRangeClamped` _returnvalue_pitch 85.0 -85.0 30.0 -120.0) _returnvalue_yaw)))

(fn `GetRightElbowOrientation`
  (params (body :type "FLKinect_Body Structure"))
  (returns (Rotator :type "Rotator Structure"))
  (bind _returnvalue (`KismetMathLibrary.Normal` (1.0 1.0 0.0)))
  (bind (_returnvalue_roll _returnvalue_pitch _returnvalue_yaw) (`KismetMathLibrary.BreakRotator` (`KismetMathLibrary.Conv_VectorToRotator` (- (- (* (`KinectPluginFunctionLibrary.GetJointPosition` body "ElbowRight") _returnvalue) (* (`KinectPluginFunctionLibrary.GetJointPosition` body "WristRight") _returnvalue)) (- (* (`KinectPluginFunctionLibrary.GetJointPosition` body "ElbowRight") _returnvalue) (* (`KinectPluginFunctionLibrary.GetJointPosition` body "ShoulderRight") _returnvalue))))))
  (return (`KismetMathLibrary.MakeRotator` 0.0 (`KismetMathLibrary.MapRangeClamped` _returnvalue_yaw 170.0 100.0 90.0 200.0))))

(fn `GetRightLegOrientation`
  (params (body :type "FLKinect_Body Structure (by ref)"))
  (returns (ReturnValue :type "Rotator Structure"))
  (bind _returnvalue (`KismetMathLibrary.Normal` (1.0 0.0 1.0)))
  (bind (_returnvalue_roll _returnvalue_pitch _returnvalue_yaw) (`KismetMathLibrary.BreakRotator` (`KismetMathLibrary.FindLookAtRotation` (* (`KinectPluginFunctionLibrary.GetJointPosition` body "HipRight") _returnvalue) (* (`KinectPluginFunctionLibrary.GetJointPosition` body "KneeRight") _returnvalue))))
  (return (`KismetMathLibrary.MakeRotator` _returnvalue_roll (`KismetMathLibrary.MapRangeClamped` _returnvalue_pitch -85.0 -20.0 0.0 40.0) _returnvalue_yaw)))

(fn `GetRightShoulderOrientation`
  (params (Body :type "FLKinect_Body Structure"))
  (returns (ReturnValue :type "Rotator Structure"))
  (bind _returnvalue (`KismetMathLibrary.Normal` (1.0 1.0 0.0)))
  (bind (_returnvalue_roll _returnvalue_pitch _returnvalue_yaw) (`KismetMathLibrary.BreakRotator` (`KismetMathLibrary.FindLookAtRotation` (`KismetMathLibrary.ProjectVectorOnToPlane` (`KinectPluginFunctionLibrary.GetJointPosition` Body "ElbowRight") _returnvalue) (`KismetMathLibrary.ProjectVectorOnToPlane` (`KinectPluginFunctionLibrary.GetJointPosition` Body "ShoulderRight") _returnvalue))))
  (return (`KismetMathLibrary.MakeRotator` _returnvalue_roll (`KismetMathLibrary.MapRangeClamped` _returnvalue_pitch 55.0 -73.0 -15.0 -140.0) _returnvalue_yaw)))

(fn `UpdateMeshLocation`
  (params (JointType :type "EFLKinect_JointType Enum") (Mesh :type "SceneComponent Object Reference") (TextCoord :type "TextRenderComponent Object Reference"))
  (`/Engine/EditorBlueprintResources/StandardMacros.IsValid` Mesh
    (:`Is Valid`
      (`SceneComponent.K2_SetRelativeLocation` Mesh (* (`KinectPluginFunctionLibrary.GetJointPosition` (`self.KinectBody`) JointType) (1.0 0.0 1.0)) false false))))

(fn `UpdateMeshOrientation`
  (params (type :type "EFLKinect_JointType Enum") (InputPin :type "SceneComponent Object Reference"))
  (`/Engine/EditorBlueprintResources/StandardMacros.IsValid` InputPin
    (:`Is Valid`
      (`SceneComponent.K2_SetWorldRotation` InputPin (`KinectPluginFunctionLibrary.GetJointOrientation` (`self.KinectBody`) type) false false))))

(fn `UserConstructionScript`)