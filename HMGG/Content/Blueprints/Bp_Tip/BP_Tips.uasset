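; BP_Tips is a tip actor that displays one of three sprites and can be shown or hidden.
; SetTipStep swaps the Tip component's sprite by state, and the construction script applies the State1 variable as the initial step.
; ShowTips sets visibility on the Root component and propagates it to its children.
; The event graph holds only empty events, so changes after construction depend on calls to these functions.
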(fn `SetTipStep`
  (params (state :type "/Game/Blueprints/Bp_Tip/Enu_TipState Enum"))
  (switch `/Game/Blueprints/Bp_Tip/Enu_TipState` state
    (:`NewEnumerator0`
      (`PaperSpriteComponent.SetSprite` (`self.tip`) (`self.State1`)))
    (:`NewEnumerator1`
      (`PaperSpriteComponent.SetSprite` (`self.tip`) (`self.State2`)))
    (:`NewEnumerator2`
      (`PaperSpriteComponent.SetSprite` (`self.tip`) (`self.State3`)))))

(fn `ShowTips`
  (params (bVisibility :type Boolean))
  (`SceneComponent.SetVisibility` (`self.Root`) bVisibility true))

(fn `UserConstructionScript`
  (`self.SetTipStep` "NewEnumerator0"))